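; Gameplay ability that dashes the Colorbound character toward the furthest location along a path.
; On activation it notifies dash start, runs a root motion MoveToForce task for the dash duration, clamping exit velocity to max speed, and fires the dash gameplay cue.
; Dash stop is called when the task times out.
; The ability itself ends separately on input release, after a zero-second delay that prevents immediately canceling into another action.
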(event `self.K2_ActivateAbility`
  (`self.CharacterDashStart`)
  (`AbilityTask_ApplyRootMotionMoveToForce.ApplyRootMotionMoveToForce` "Dashing" (`self.GetFurthestLocationAlongPath`) (`self.DashDuration`) false "MOVE_None" false null "ClampVelocity" (0.0 0.0 0.0) (`MovementComponent.GetMaxSpeed` (`Pawn.GetMovementComponent` (`self.GetColorboundCharacterFromActorInfo`)))
    (:`then`
      (`self.K2_ExecuteGameplayCueWithParams` (struct :`TagName` "GameplayCue.Ability.Dash") (`AbilitySystemBlueprintLibrary.MakeGameplayCueParameters` (`self.DashDuration`) (`self.MaxDashDistance`) (struct) (struct) (struct) (struct) (struct) (`Actor.K2_GetActorLocation` (`self.GetColorboundCharacterFromActorInfo`))))
      (`AbilityTask_WaitInputRelease.WaitInputRelease` false
        (:`OnRelease`
          ;[1 1 1] Delay end of ability so you can't immediately cancel into another action
          (`KismetSystemLibrary.Delay` 0.0)
          (`self.K2_EndAbility`))))
    (:`OnTimedOut`
      (`self.CharacterDashStop` :!label _label))
    (:`OnTimedOutAndDestinationReached`
      (goto _label))))