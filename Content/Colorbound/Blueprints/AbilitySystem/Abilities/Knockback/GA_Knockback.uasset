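; Gameplay ability that knocks a Colorbound character back when activated.
; It derives the horizontal push direction from the hit result in the granting effect's context, from trace start to hit location.
; It turns the character opposite the push, then applies a root motion constant force using Height as the vertical component and Strength as magnitude.
; The ability ends when the force finishes, maintaining the last root motion velocity.
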(event `self.K2_ActivateAbility`
  (bind (_direction_x _direction_y) (`KismetMathLibrary.BreakVector2D` (`self.Direction`)))
  (bind (_returnvalue_x _returnvalue_y) (`KismetMathLibrary.BreakVector2D` (* (`self.Direction`) -1.0)))
  (set `self.Direction` (`self.GetImpulseDirection`))
  (`ColorboundCharacterBase.SetDirectionality` (`self.GetColorboundCharacterFromActorInfo`) (`KismetMathLibrary.MakeVector2D` _returnvalue_x _returnvalue_y))
  (`AbilityTask_ApplyRootMotionConstantForce.ApplyRootMotionConstantForce` "Knockback" (`KismetMathLibrary.MakeVector` _direction_x _direction_y (`self.Height`)) (`self.Strength`) 0.0 false null "MaintainLastRootMotionVelocity"
    (:`OnFinish`
      (`self.K2_EndAbility`))))

(fn `GetImpulseDirection`
  (returns (Direction :type "Vector2D Structure"))
  (bind (_bblockinghit _binitialoverlap _time _distance _location _impactpoint _normal _impactnormal _physmat _hitactor _hitcomponent _hitbonename _bonename _hititem _elementindex _faceindex _tracestart) (`GameplayStatics.BreakHitResult` (`AbilitySystemBlueprintLibrary.EffectContextGetHitResult` (`self.GetGrantedByEffectContext`))))
  (bind (_returnvalue_x _returnvalue_y) (`KismetMathLibrary.BreakVector` (- _location _tracestart)))
  (return (`KismetMathLibrary.MakeVector2D` _returnvalue_x _returnvalue_y)))