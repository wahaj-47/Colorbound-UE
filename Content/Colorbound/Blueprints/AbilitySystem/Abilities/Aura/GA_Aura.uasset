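; Gameplay ability that gives its owner an aura, applying a gameplay effect to actors while they overlap it.
; It adds the aura component when granted, then on activation runs a WaitOverlap task on that component.
; Begin overlap applies the configured effect class to the actor.
; End overlap removes effects by that class's asset tags, so other active effects matching those tags are also removed.
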(event `self.K2_OnAbilityAdded`
  (`self.AddAuraComponent`))

(event `self.K2_ActivateAbility`
  (bind (_asynctaskproxy _overlappedactor) (`WaitOverlap.WaitOverlap` null (`self.AuraComponent`))
    (:`OnBeginOverlap`
      (`self.BP_ApplyGameplayEffectToTarget` (`AbilitySystemBlueprintLibrary.AbilityTargetDataFromActor` _overlappedactor) (`self.AuraEffectClass`)))
    (:`OnEndOverlap`
      (`AbilitySystemComponent.RemoveActiveEffectsWithTags` (`AbilitySystemBlueprintLibrary.GetAbilitySystemComponent` _overlappedactor) (`AbilitySystemBlueprintLibrary.GetGameplayEffectAssetTags` (`self.AuraEffectClass`))))))