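; BP_CameraActor is a shared camera that keeps all BP_PlayerCharacter actors framed together.
; It caches the players one tick after BeginPlay, then computes their colliding-component bounds every Tick.
; It lerps toward the bounds center with a frame-rate-dependent alpha and maps the larger X/Y extent to boom arm length.
; Both movement and zoom pause while either extent reaches or exceeds its maximum.
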(event `self.ReceiveBeginPlay`
  (`KismetSystemLibrary.Delay` 0.0)
  (bind _outactors (`GameplayStatics.GetAllActorsOfClass` "/Game/Colorbound/Blueprints/Core/BP_PlayerCharacter.BP_PlayerCharacter_C"))
  (set `self.PlayerCharacters` _outactors))

(event `self.ReceiveTick`
  (params (DeltaSeconds :type "Float (single-precision)"))
  (bind (_center _boxextent) (`GameplayStatics.GetActorArrayBounds` (`self.PlayerCharacters`) true))
  (if (and (< (.x _boxextent) (`self.MaxX`)) (< (.y _boxextent) (`self.MaxY`)))
    (`self.Move` _center)
    (`self.Zoom` _boxextent)))

(fn `Move`
  (params (Center :type "Vector Structure"))
  (`self.K2_SetActorLocation` (`KismetMathLibrary.VLerp` (`self.K2_GetActorLocation`) Center (`self.FollowSpeed`))))

(fn `UserConstructionScript`)

(fn `Zoom`
  (params (BoxExtent :type "Vector Structure"))
  (locals (CurrentPlayer :type "/Game/Colorbound/Blueprints/Core/BP_PlayerCharacter Object Reference") (MinTargetArmLength :type "Float (double-precision)" :default 300.0) (MaxTargetArmLength :type "Float (double-precision)" :default 800.0) (MaxPlayerDistance :type "Float (double-precision)" :default 300.0))
  (set `SpringArmComponent.TargetArmLength` (`KismetMathLibrary.Lerp` (`local.MinTargetArmLength`) (`local.MaxTargetArmLength`) (`KismetMathLibrary.MapRangeClamped` (`KismetMathLibrary.FMax` BoxExtent_X BoxExtent_Y) 60.0 (`local.MaxPlayerDistance`) 0.0 1.0)) (`self.CameraBoom`)))