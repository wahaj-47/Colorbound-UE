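; BP_EnemyCharacter is the enemy character Blueprint, handling its health bar display and death sequence.
; On BeginPlay it creates a health bar widget, binds it to the current health view model from CharacterViewModel and assigns it to the HealthBar component.
; StartDeathTimeline plays a timeline that toggles sprite visibility for a flicker effect, then returns the enemy to its pool when finished instead of destroying it.
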(event `self.ReceiveBeginPlay`
  (bind _returnvalue (`|CreateWidget` "/Game/Colorbound/Blueprints/UI/Health/WBP_HealthBar.WBP_HealthBar_C" null null))
  (`/Game/Colorbound/Blueprints/UI/Health/WBP_HealthBar.SetViewModel_Health` _returnvalue (`ViewModel_Character.CurrentHealthViewModel` (`self.CharacterViewModel`)))
  (`WidgetComponent.SetWidget` (`self.HealthBar`) _returnvalue))

(event `self.StartDeathTimeline`
  (`Timeline|Death Timeline` :!via `PlayFromStart`
    (:`Finished`
      (`|ReturnToPool` self))
    (:`Toggle`
      (`SceneComponent.ToggleVisibility` (`self.Sprite`) false))))

(fn `UserConstructionScript`)